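; BP_MovingTrap is a trap actor whose Cylinder component shuttles endlessly between two target actors, Target1 and Target2.
; From BeginPlay, two MoveComponentTo latent moves run in sequence and loop back, each lasting a fixed short time.
; Each target's world transform is converted into the trap's relative space to get the move destination.
; Overlap and Tick events are empty, so the file contains only the motion.
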(event `self.ReceiveBeginPlay`
  (bind _returnvalue_location (`KismetMathLibrary.BreakTransform` (`KismetMathLibrary.MakeRelativeTransform` (`self.GetTransform` (`self.Target2`)) (`self.GetTransform`))))
  (bind _returnvalue_location_2 (`KismetMathLibrary.BreakTransform` (`KismetMathLibrary.MakeRelativeTransform` (`self.GetTransform` (`self.Target1`)) (`self.GetTransform`))))
  (`KismetSystemLibrary.MoveComponentTo` (`self.Cylinder`) _returnvalue_location_2 (struct) false false 0.7 :!label _label)
  (`KismetSystemLibrary.MoveComponentTo` (`self.Cylinder`) _returnvalue_location (struct) false false 0.7)
  (goto _label))

(fn `UserConstructionScript`)