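; BP_Rejas is a trap whose Lava component moves between Start and Goal positions and applies damage to actors that overlap its collision box.
; ActivateLava waits briefly, plays a sound, moves the component to Goal, then after another delay calls DeactivateLava to return it to Start.
; The damage overlap runs independently of that cycle, and nothing in this Blueprint calls ActivateLava.
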(event `Activate Lava`
  (`KismetSystemLibrary.Delay` 0.5)
  (`GameplayStatics.PlaySound2D` "/Game/Sound/SW_Rejas.SW_Rejas" 1.0 1.0 0.3 null null)
  (`KismetSystemLibrary.MoveComponentTo` (`self.Lava`) (`SceneComponent.RelativeLocation` (`self.Goal`)))
  (`KismetSystemLibrary.Delay` 0.5)
  (`self.Deactivate Lava`))

(event `Deactivate Lava`
  (`KismetSystemLibrary.MoveComponentTo` (`self.Lava`) (`SceneComponent.RelativeLocation` (`self.Start`))))

(event `self.BoxColl.OnComponentBeginOverlap`
  (params (OverlappedComponent :type "PrimitiveComponent Object Reference") (OtherActor :type "Actor Object Reference") (OtherComp :type "PrimitiveComponent Object Reference") (OtherBodyIndex :type Integer) (bFromSweep :type Boolean) (SweepResult :type "HitResult Structure (by ref)"))
  (`GameplayStatics.ApplyDamage` OtherActor))

(fn `UserConstructionScript`)