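; BP_enemyPush is an enemy actor that launches the third-person player character when it overlaps HitCollision.
; The launch follows the normalized vector from character to enemy, scaled by PushForce, adding to horizontal velocity and replacing vertical.
; GetDamage subtracts from CurrentLife and broadcasts the life change.
; GetEnergy does nothing, as its energy-change broadcast is disconnected.
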(event `self.HitCollision.OnComponentBeginOverlap`
  (params (OverlappedComponent :type "PrimitiveComponent Object Reference") (OtherActor :type "Actor Object Reference") (OtherComp :type "PrimitiveComponent Object Reference") (OtherBodyIndex :type Integer) (bFromSweep :type Boolean) (SweepResult :type "HitResult Structure (by ref)"))
  (bind _asbp_third_person_character (cast `/Game/ThirdPerson/Blueprints/BP_ThirdPersonCharacter` OtherActor))
  (`self.LaunchCharacter` _asbp_third_person_character (* (`KismetMathLibrary.Normal` (- (`self.K2_GetActorLocation`) (`self.K2_GetActorLocation` _asbp_third_person_character))) (`self.PushForce`)) false true))

(fn `GetDamage`
  (params (InDamage :type "Float (double-precision)"))
  (set `self.CurrentLife` (- (`self.CurrentLife`) InDamage))
  (`self.OnLifeChange` (`self.CurrentLife`) (`self.MaxLife`)))

(fn `GetEnergy`
  (params (InEnergy :type "Float (double-precision)"))
  (locals (NewLocalVar :type "Float (double-precision)") (`Current Energy` :type "Float (double-precision)")))

(fn `UserConstructionScript`)