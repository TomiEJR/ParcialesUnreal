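; BP_Enemi3 is an enemy actor that configures itself from a data table and reports player sightings to its AI.
; On BeginPlay it reads the "Enemigo3" row of EnemieDataTable, storing SightRange and passing Health to BPHealthComponent.
; AI perception updates for BP_ThirdPersonCharacter write the player to a Blackboard key when sensed, and clear it otherwise.
; SightRange is only stored here, not applied to the perception component.
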(event `self.ReceiveBeginPlay`
  (bind _returnvalue (`|GetDataTableRow` "/Game/Struct/EnemieDataTable.EnemieDataTable" "Enemigo3")
    (:`then`
      (bind (_sightrange _health) (break `/Game/Struct/DT_Enemies` _returnvalue))
      (set `self.SightRange` _sightrange)
      (`/Game/ActorComponents/BP_HealthComponent.SetHealth` (`self.BP_HealthComponent`) _health))))

(event `self.AIPerception.OnTargetPerceptionUpdated`
  (params (Actor :type "Actor Object Reference") (Stimulus :type "AIStimulus Structure"))
  (bind _asbp_third_person_character (cast `/Game/ThirdPerson/Blueprints/BP_ThirdPersonCharacter` Actor))
  (`BlackboardComponent.SetValueAsObject` (`AIBlueprintHelperLibrary.GetBlackboard` (`self.GetController`)) (`self.Key Name`) (select `bool` (`.bSuccessfullySensed` (break `AIStimulus` Stimulus)) :`true` _asbp_third_person_character :!type "Object Object Reference")))

(fn `UserConstructionScript`)