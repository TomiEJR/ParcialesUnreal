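; Energy component that tracks a current and maximum energy value for its owner.
; BeginPlay fills energy to the maximum and broadcasts OnEnergyChange with both values.
; GetEnergy, despite its name, subtracts energy without a lower bound and broadcasts the change.
; AddEnergy sets energy to MaxEnergy when the sum exceeds a hardcoded 100 rather than MaxEnergy, and does not broadcast.
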(event `self.ReceiveBeginPlay`
  (bind _output_get (set `self.CurrentEnergy` (`self.MaxEnergy`)))
  (`self.On Energy Change` _output_get (`self.MaxEnergy`)))

(fn `AddEnergy`
  (params (EnergyAdd :type "Float (double-precision)"))
  (bind _returnvalue (+ EnergyAdd (`self.CurrentEnergy`)))
  (if (> _returnvalue 100.0)
    (set `self.CurrentEnergy` (`self.MaxEnergy`))
    (else
      (set `self.CurrentEnergy` _returnvalue))))

(fn `GetEnergy`
  (params (`In Energy` :type "Float (double-precision)"))
  (bind _output_get (set `self.CurrentEnergy` (- (`self.CurrentEnergy`) `In Energy`)))
  (`self.On Energy Change` _output_get (`self.MaxEnergy`)))