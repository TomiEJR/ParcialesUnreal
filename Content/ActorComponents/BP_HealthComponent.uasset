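; Health component that tracks an owning actor's life, starting it at MaxLife on BeginPlay.
; Healing and damage clamp life between zero and MaxLife, while SetHealth assigns it unclamped; every change broadcasts OnLifeChange with current and max values.
; Damage that leaves life at zero broadcasts OnDeath.
; A separate Die function, not called within the component, opens the lose level and destroys the owner.
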(event `self.ReceiveBeginPlay`
  (`self.Initialize`))

(fn `AddLife`
  (params (HealingAmount :type "Float (double-precision)"))
  (set `self.CurrentLife` (`KismetMathLibrary.FClamp` (+ HealingAmount (`self.CurrentLife`)) 0.0 (`self.MaxLife`)))
  (`self.LifeChange`))

(fn `Die`
  (`GameplayStatics.OpenLevelBySoftObjectPtr` "/Game/LoseLevel/Map_LoseLevel.Map_LoseLevel")
  (`Actor.K2_DestroyActor` (`self.GetOwner`)))

(fn `Get Dmg`
  (params (InDamage :type "Float (double-precision)"))
  (bind _output_get (set `self.CurrentLife` (`KismetMathLibrary.FClamp` (- (`self.CurrentLife`) InDamage) 0.0 (`self.MaxLife`))))
  (`self.LifeChange`)
  (if (<= _output_get 0.0)
    (`self.OnDeath`)))

(fn `GetLife`
  (returns (CurrentHealth :type "Float (double-precision)"))
  (return (`self.CurrentLife`)))

(fn `Initialize`
  (set `self.CurrentLife` (`self.MaxLife`))
  (`self.LifeChange`))

(fn `IsAlive`
  (returns (IsAlive :type Boolean))
  (return (> (`self.CurrentLife`) 0.0)))

(fn `LifeChange`
  (`self.OnLifeChange` (`self.CurrentLife`) (`self.MaxLife`)))

(fn `SetHealth`
  (params (CurrentLife :type "Float (double-precision)"))
  (set `self.CurrentLife` CurrentLife)
  (`self.LifeChange`))