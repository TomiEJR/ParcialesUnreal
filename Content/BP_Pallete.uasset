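; Pallet actor that changes color saturation, vanishes and later reappears after the third-person character enters its trigger box.
; BeginPlay creates a dynamic material instance with zero saturation, which a timeline animates on overlap.
; Delays chained from that timeline's Update hide the mesh and disable collision, then show it again.
; A second timeline, played in reverse, drives saturation and sets collision to query-only rather than physics collision.
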(event `self.ReceiveBeginPlay`
  (bind _returnvalue (`KismetMaterialLibrary.CreateDynamicMaterialInstance` (`PrimitiveComponent.GetMaterial` (`self.SM_Pallet`) 0)))
  (bind _output_get (set `self.NewVar` _returnvalue))
  (`PrimitiveComponent.SetMaterial` (`self.SM_Pallet`) 0 _output_get)
  (`MaterialInstanceDynamic.SetScalarParameterValue` (`self.NewVar`) "Saturation" 0.0))

(event `self.Box.OnComponentBeginOverlap`
  (params (OverlappedComponent :type "PrimitiveComponent Object Reference") (OtherActor :type "Actor Object Reference") (OtherComp :type "PrimitiveComponent Object Reference") (OtherBodyIndex :type Integer) (bFromSweep :type Boolean) (SweepResult :type "HitResult Structure (by ref)"))
  (cast `/Game/ThirdPerson/Blueprints/BP_ThirdPersonCharacter` OtherActor)
  (bind (_direction _1) (`Timeline|Timeline`)
    (:`Update`
      (`MaterialInstanceDynamic.SetScalarParameterValue` (`self.NewVar`) "Saturation" _1)
      (`KismetSystemLibrary.Delay` 1.0)
      (`SceneComponent.SetVisibility` (`self.SM_Pallet`) false false)
      (`PrimitiveComponent.SetCollisionEnabled` (`self.SM_Pallet`) "NoCollision")
      (`KismetSystemLibrary.Delay` 3.0)
      (`SceneComponent.SetVisibility` (`self.SM_Pallet`) true false)
      (bind (_direction_2 _1_2) (`Timeline|Timeline_0` :!via `Reverse`)
        (:`Update`
          (`MaterialInstanceDynamic.SetScalarParameterValue` (`self.NewVar`) "Saturation" _1_2)
          (`PrimitiveComponent.SetCollisionEnabled` (`self.SM_Pallet`) "QueryOnly"))))))

(event `self.Box.OnComponentEndOverlap`
  (params (OverlappedComponent :type "PrimitiveComponent Object Reference") (OtherActor :type "Actor Object Reference") (OtherComp :type "PrimitiveComponent Object Reference") (OtherBodyIndex :type Integer)))

(fn `UserConstructionScript`)